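; BP_Dark_Fairy is a collectible fairy that hovers via a timeline from BeginPlay until the RunnerCharacter overlaps it.
; Overlap flags fairy 3 as collected in StarChaserGameMode, saves, and plays a second timeline that moves it along Z to fly away.
; That timeline's update fires a one-time pickup sound and, with five or more fairies found, unlocks the "Better Together" bright star, adding 100 stars and saving.
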(event EventBeginPlay
  (bind _returnvalue (Transformation|GetActorLocation))
  ;[1 1 1] Fairy Spawn Movement
  (bind _hovering (Timeline|Timeline_2 Play)
    (:Update
      (Transformation|SetActorLocation (Math|Vector|MakeVector (.x _returnvalue) (.y _returnvalue) (+ (.z _returnvalue) _hovering)) false false))))

(event Collision|EventActorBeginOverlap
  (params (OtherActor :type Actor%20Object%20Reference))
  (bind _returnvalue (Transformation|GetActorLocation))
  ;[1 1 1] Update Saved File
  (Utilities|Casting|CastToRunnerCharacter OtherActor)
  (bind _asstar_chaser_game_mode (Utilities|Casting|CastToStarChaserGameMode (Game|GetGameMode)))
  (Class|StarChaserGameMode|SetFairyTrue _asstar_chaser_game_mode 3)
  (Class|StarChaserGameMode|Save _asstar_chaser_game_mode)
  ;[1 1 1] Fairy Fly Away
  (bind _newtrack_0 (Timeline|Timeline_0 Play)
    (:Update
      (Transformation|SetActorLocation (Math|Vector|MakeVector (.x _returnvalue) (.y _returnvalue) (+ (.z _returnvalue) _newtrack_0)) false false)
      (Utilities|Casting|CastToRotatingMovementComponent (Variables|Default|GetRotatingMovement))
      (Utilities|FlowControl|DoOnce false
        (:Completed
          (Audio|PlaySound2D "/Game/Audio/FairyPickup2.FairyPickup2" 1.0 1.0 0.0 0 0)
          ;[1 1 1] Better Together Bright Star
          (bind _asstar_chaser_game_mode_2 (Utilities|Casting|CastToStarChaserGameMode (Game|GetGameMode)))
          (bind _returnvalue_2 (Class|StarChaserGameMode|FairiesCounter _asstar_chaser_game_mode_2))
          (if (>= _returnvalue_2 5)
            (bind _returnvalue_3 (Class|StarChaserGameMode|GetBrightStarActive _asstar_chaser_game_mode_2 3))
            (if (not _returnvalue_3)
              (Class|StarChaserGameMode|SetBrightStarTrue _asstar_chaser_game_mode_2 3)
              (bind _returnvalue_4 (Class|StarChaserGameMode|GetTotalStars _asstar_chaser_game_mode_2))
              (Class|StarChaserGameMode|SetTotalStars _asstar_chaser_game_mode_2 (+ _returnvalue_4 100))
              (Class|StarChaserGameMode|Save _asstar_chaser_game_mode_2))))))))

(fn ConstructionScript)
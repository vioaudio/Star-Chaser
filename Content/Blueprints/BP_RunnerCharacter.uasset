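; BP_RunnerCharacter is the runner-mode player character, handling skin selection and runner UI.
; On BeginPlay it reads StarChaserGameMode to apply the Nova skin and, if the runner is running, shows the runner HUD with brief fairy count and reminder widgets.
; A collapsed number-key graph funnels digit, plus and minus presses into a DoOnce that re-shows those two timed widgets without stacking.
; Escape calls Death.
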(event EventBeginPlay
  (bind _asstar_chaser_game_mode (Utilities|Casting|CastToStarChaserGameMode (Game|GetGameMode)))
  (if (Variables|/Script/StarChaser_C.StarChaserGameMode|GetbNovaSkin _asstar_chaser_game_mode)
    (Class|SkinnedMeshComponent|SetSkeletalMesh (Variables|Character|GetMesh) "/Game/Mannequin/Character/Mesh/SK_NovaSkin.SK_NovaSkin" true))
  ;[1 1 1] Runner HUD
  (bind _asstar_chaser_game_mode_2 (Utilities|Casting|CastToStarChaserGameMode (Game|GetGameMode)))
  (Development|PrintString (Utilities|String|ToString(Boolean) (Variables|/Script/StarChaser_C.StarChaserGameMode|GetbRunnerRunning _asstar_chaser_game_mode_2)))
  (if (Variables|/Script/StarChaser_C.StarChaserGameMode|GetbRunnerRunning _asstar_chaser_game_mode_2)
    (bind _returnvalue (UserInterface|CreateWidget "/Game/Blueprints/UI/WBP_FairyCount.WBP_FairyCount_C"))
    (bind _returnvalue_2 (UserInterface|CreateWidget "/Game/Blueprints/UI/WBP_Reminder.WBP_Reminder_C"))
    (bind _returnvalue_3 (UserInterface|CreateWidget "/Game/Blueprints/UI/WBP_RunnerHUD.WBP_RunnerHUD_C"))
    (UserInterface|Viewport|AddtoViewport _returnvalue_3 0)
    (Utilities|FlowControl|Delay 7.0)
    (Widget|RemovefromParent _returnvalue)))

(event Input|KeyboardEvents|Escape
  (params (Key :type Key%20Structure :default "None"))
  (:Pressed
    (Class|RunnerCharacter|Death)))

(fn ConstructionScript)

(event Input|KeyboardEvents|1
  (params (Key :type Key%20Structure :default "None"))
  (:Pressed
    (return)))

(event Input|KeyboardEvents|2
  (params (Key :type Key%20Structure :default "None"))
  (:Pressed
    (|Outputs) ; enters at Pressed2
  ))

(event Input|KeyboardEvents|9
  (params (Key :type Key%20Structure :default "None"))
  (:Pressed
    (|Outputs) ; enters at Pressed9
  ))

(event Input|KeyboardEvents|0
  (params (Key :type Key%20Structure :default "None"))
  (:Pressed
    (|Outputs) ; enters at Pressed10
  ))

(event Input|KeyboardEvents|Subtract
  (params (Key :type Key%20Structure :default "None"))
  (:Pressed
    (|Outputs) ; enters at Pressed11
  ))

(event Input|KeyboardEvents|Add
  (params (Key :type Key%20Structure :default "None"))
  (:Pressed
    (|Outputs) ; enters at Pressed12
  ))

(event Input|KeyboardEvents|3
  (params (Key :type Key%20Structure :default "None"))
  (:Pressed
    (|Outputs) ; enters at Pressed3
  ))

(event Input|KeyboardEvents|4
  (params (Key :type Key%20Structure :default "None"))
  (:Pressed
    (|Outputs) ; enters at Pressed4
  ))

(event Input|KeyboardEvents|5
  (params (Key :type Key%20Structure :default "None"))
  (:Pressed
    (|Outputs) ; enters at Pressed5
  ))

(event Input|KeyboardEvents|6
  (params (Key :type Key%20Structure :default "None"))
  (:Pressed
    (|Outputs) ; enters at Pressed6
  ))

(event Input|KeyboardEvents|7
  (params (Key :type Key%20Structure :default "None"))
  (:Pressed
    (|Outputs) ; enters at Pressed7
  ))

(event Input|KeyboardEvents|8
  (params (Key :type Key%20Structure :default "None"))
  (:Pressed
    (|Outputs) ; enters at Pressed8
  ))
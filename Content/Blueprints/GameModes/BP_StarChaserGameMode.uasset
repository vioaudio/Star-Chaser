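; BP_StarChaserGameMode is the game mode Blueprint that handles startup for the StarChaser game.
; On BeginPlay it spawns the first tile at the origin, then checks RunnerRunning on the current StarChaserGameMode.
; A running runner fades in the game music; otherwise it prints a debug string and shows the black background and main menu widgets.
; Tick forces the mouse cursor visible every frame.
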(event EventBeginPlay
  (Game|SpawnActorfromClass "/Game/Blueprints/FloorTiles/BP_FirstTile.BP_FirstTile_C" (Variables|Default|GetOrigin) "Undefined" 0 0)
  (bind _asstar_chaser_game_mode (Utilities|Casting|CastToStarChaserGameMode (Game|GetGameMode)))
  (if (Variables|/Script/StarChaser_C.StarChaserGameMode|GetbRunnerRunning _asstar_chaser_game_mode)
    (Class|StarChaserGameMode|FadeinGameMusic _asstar_chaser_game_mode)
    (else
      (Development|PrintString "Runnner Running Was False")
      (bind _returnvalue (UserInterface|CreateWidget "/Game/Blueprints/UI/WBP_BlackBackground.WBP_BlackBackground_C"))
      (UserInterface|Viewport|AddtoViewport _returnvalue 0)
      (bind _returnvalue_2 (UserInterface|CreateWidget "/Game/Blueprints/UI/WBP_MainMenu.WBP_MainMenu_C"))
      (UserInterface|Viewport|AddtoViewport _returnvalue_2 0))))

(event EventTick
  (params (DeltaSeconds :type Float%20%28single-precision%29))
  (Variables|/Script/Engine.PlayerController|SetbShowMouseCursor (Game|GetPlayerController 0) true))

(fn ConstructionScript)
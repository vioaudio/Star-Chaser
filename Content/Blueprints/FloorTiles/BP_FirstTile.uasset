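; Opening floor tile with a three-lane spawner for hurdles, boxes, stars, magnet and boots pickups.
; Tick polls a collision component for WorldDynamic overlaps and spawns one bright star, guarded by a counter, with a debug print.
; SpawnObstacles, not called here, cascades range checks per lane, each rerolling its random value.
; Later lanes run only after the previous one spawns something, so a failed cascade skips them.
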(event EventBeginPlay)

(event EventTick
  (params (DeltaSeconds :type Float%20%28single-precision%29))
  (bind _counter (Variables|Default|GetCounter))
  (bind _brightstarcollision1 (Variables|Default|GetBrightStarCollision1))
  (bind _returnvalue (Collision|ComponentOverlapActors _brightstarcollision1 (Transformation|GetWorldTransform _brightstarcollision1) (Utilities|Array|MakeArray "ObjectTypeQuery2") 0))
  (if _returnvalue
    (if (< _counter 1)
      (Development|PrintString "Hello")
      (Game|SpawnActorfromClass "/Game/Blueprints/BrightStars/BP_BrightStar1.BP_BrightStar1_C" (Variables|Default|GetBS%20Spawn) "Undefined" 0 0)
      (Math|Integer|IncrementInt _counter))))

(fn ConstructionScript)

(fn SpawnObstacles
  (bind _returnvalue (Math|Random|RandomFloatinRange 0.0 1.0))
  (bind _returnvalue_2 (Math|Random|RandomFloatinRange 0.0 1.0))
  (bind _returnvalue_3 (Math|Random|RandomFloatinRange 0.0 1.0))
  (bind _lane0 (Variables|Default|GetLane0))
  (bind _lane1 (Variables|Default|GetLane1))
  (bind _lane2 (Variables|Default|GetLane2))
  (bind _returnvalue_4 (Transformation|GetWorldTransform _lane0))
  (bind _returnvalue_5 (Transformation|GetWorldTransform _lane2))
  (bind _returnvalue_6 (Transformation|GetWorldTransform _lane1))
  ;[1 1 1] LANE0
  (if (Math|Float|InRange(Float) _returnvalue_2 0.0 0.4)
    (Game|SpawnActorfromClass "/Game/Blueprints/Obstacles/BP_Obstacle_Hurdle.BP_Obstacle_Hurdle_C" _returnvalue_4 "Undefined" 0 0)
    ;[1 1 1] LANE1
    (if (Math|Float|InRange(Float) _returnvalue_3 0.0 0.4) :!label _label
      (Game|SpawnActorfromClass "/Game/Blueprints/Obstacles/BP_Obstacle_Hurdle.BP_Obstacle_Hurdle_C" _returnvalue_6 "Undefined" 0 0)
      ;[1 1 1] LANE2
      (if (Math|Float|InRange(Float) _returnvalue 0.0 0.4) :!label _label_2
        (Game|SpawnActorfromClass "/Game/Blueprints/Obstacles/BP_Obstacle_Hurdle.BP_Obstacle_Hurdle_C" _returnvalue_5 "Undefined" 0 0)
        (elif (Math|Float|InRange(Float) _returnvalue 0.4 0.5)
          (Game|SpawnActorfromClass "/Game/Blueprints/Obstacles/BP_Obstacle_Box.BP_Obstacle_Box_C" _returnvalue_5 "Undefined" 0 0)
          (elif (Math|Float|InRange(Float) _returnvalue 0.5 0.95)
            (Game|SpawnActorfromClass "/Game/Blueprints/PowerUps/BP_StarPickUp.BP_StarPickUp_C" _returnvalue_5 "Undefined" 0 0)
            (elif (Math|Float|InRange(Float) _returnvalue 0.95 0.975)
              (Game|SpawnActorfromClass "/Game/Blueprints/PowerUps/BP_MagnetPickup.BP_MagnetPickup_C" _returnvalue_5 "Undefined" 0 0)
              (elif (Math|Float|InRange(Float) _returnvalue 0.975 1.0)
                (Game|SpawnActorfromClass "/Game/Blueprints/PowerUps/BP_BootsPickUp.BP_BootsPickUp_C" _returnvalue_5 "Undefined" 0 0))))))
      (elif (Math|Float|InRange(Float) _returnvalue_3 0.4 0.5)
        (Game|SpawnActorfromClass "/Game/Blueprints/Obstacles/BP_Obstacle_Box.BP_Obstacle_Box_C" _returnvalue_6 "Undefined" 0 0)
        (goto _label_2)
        (elif (Math|Float|InRange(Float) _returnvalue_3 0.5 0.95)
          (Game|SpawnActorfromClass "/Game/Blueprints/PowerUps/BP_StarPickUp.BP_StarPickUp_C" _returnvalue_6 "Undefined" 0 0)
          (goto _label_2)
          (elif (Math|Float|InRange(Float) _returnvalue_3 0.95 0.975)
            (Game|SpawnActorfromClass "/Game/Blueprints/PowerUps/BP_MagnetPickup.BP_MagnetPickup_C" _returnvalue_6 "Undefined" 0 0)
            (goto _label_2)
            (elif (Math|Float|InRange(Float) _returnvalue_3 0.975 1.0)
              (Game|SpawnActorfromClass "/Game/Blueprints/PowerUps/BP_BootsPickUp.BP_BootsPickUp_C" _returnvalue_6 "Undefined" 0 0)
              (goto _label_2))))))
    (elif (Math|Float|InRange(Float) _returnvalue_2 0.4 0.5)
      (Game|SpawnActorfromClass "/Game/Blueprints/Obstacles/BP_Obstacle_Box.BP_Obstacle_Box_C" _returnvalue_4 "Undefined" 0 0)
      (goto _label)
      (elif (Math|Float|InRange(Float) _returnvalue_2 0.5 0.95)
        (Game|SpawnActorfromClass "/Game/Blueprints/PowerUps/BP_StarPickUp.BP_StarPickUp_C" _returnvalue_4 "Undefined" 0 0)
        (goto _label)
        (elif (Math|Float|InRange(Float) _returnvalue_2 0.95 0.975)
          (Game|SpawnActorfromClass "/Game/Blueprints/PowerUps/BP_MagnetPickup.BP_MagnetPickup_C" _returnvalue_4 "Undefined" 0 0)
          (goto _label)
          (elif (Math|Float|InRange(Float) _returnvalue_2 0.975 1.0)
            (Game|SpawnActorfromClass "/Game/Blueprints/PowerUps/BP_BootsPickUp.BP_BootsPickUp_C" _returnvalue_4 "Undefined" 0 0)
            (goto _label)))))))
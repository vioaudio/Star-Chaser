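; BP_BrightStar5 is a collectible bright star pickup in a star-chasing game.
; On BeginPlay a Hover timeline offsets its Z position each update and also drives a Grow timeline that sets its scale.
; On overlap it marks bright star index 4 collected in StarChaserGameMode, adds to total and current star counts, and saves.
; It then plays a chime and destroys itself.
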(event EventBeginPlay
  (bind _returnvalue (Transformation|GetActorLocation))
  ;[1 1 1] BrightStar Spawn
  (bind _hovering (Timeline|Hover PlayFromStart)
    (:Update
      (Transformation|SetActorLocation (Math|Vector|MakeVector (.x _returnvalue) (.y _returnvalue) (+ (.z _returnvalue) _hovering)) false false)
      (bind _grow (Timeline|Grow Play)
        (:Update
          (Transformation|SetActorScale3D (Math|Vector|MakeVector (.x _grow) (.y _grow) (.z _grow))))))))

(event EventTick
  (params (DeltaSeconds :type Float%20%28single-precision%29)))

(event Collision|EventActorBeginOverlap
  (params (OtherActor :type Actor%20Object%20Reference))
  ;[1 1 1] Save BrightStar
  (bind _asstar_chaser_game_mode (Utilities|Casting|CastToStarChaserGameMode (Game|GetGameMode)))
  (Class|StarChaserGameMode|SetBrightStarTrue _asstar_chaser_game_mode 4)
  (bind _returnvalue (Class|StarChaserGameMode|GetTotalStars _asstar_chaser_game_mode))
  (Class|StarChaserGameMode|SetTotalStars _asstar_chaser_game_mode (+ _returnvalue 100))
  (bind _returnvalue_2 (Class|StarChaserGameMode|GetCurrentStars _asstar_chaser_game_mode))
  (Class|StarChaserGameMode|SetCurrentStars _asstar_chaser_game_mode (+ _returnvalue_2 100))
  (Class|StarChaserGameMode|Save _asstar_chaser_game_mode)
  (Audio|SpawnSound2D "/Game/Audio/chime_tinkle_wood_bell_positive_05.chime_tinkle_wood_bell_positive_05" 1.0 1.0 0.0 0)
  (Actor|DestroyActor))

(fn ConstructionScript)
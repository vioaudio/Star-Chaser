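; BP_BrightStar2 is a collectible Bright Star pickup that rewards stars when a pawn touches it.
; On BeginPlay, a Hover timeline adds a Z offset to its current location each update and also drives a Grow timeline that scales it.
; Tick polls the mesh for pawn overlaps, then flags this star in StarChaserGameMode, increases total and current star counts, saves, plays a chime and destroys itself.
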(event EventBeginPlay
  (bind _returnvalue (Transformation|GetActorLocation))
  ;[1 1 1] BrightStar Spawn
  (bind _hovering (Timeline|Hover PlayFromStart)
    (:Update
      (Transformation|SetActorLocation (Math|Vector|MakeVector (.x _returnvalue) (.y _returnvalue) (+ (.z _returnvalue) _hovering)) false false)
      (bind _grow (Timeline|Grow Play)
        (:Update
          (Transformation|SetActorScale3D (Math|Vector|MakeVector (.x _grow) (.y _grow) (.z _grow))))))))

(event EventTick
  (params (DeltaSeconds :type Float%20%28single-precision%29))
  ;[1 1 1] Collision
  (bind _returnvalue (Collision|ComponentOverlapActors (Variables|Default|GetStaticMesh) (Transformation|GetActorTransform) (Utilities|Array|MakeArray "ObjectTypeQuery3") 0))
  ;[1 1 1] Save BrightStar
  (if _returnvalue
    (bind _asstar_chaser_game_mode (Utilities|Casting|CastToStarChaserGameMode (Game|GetGameMode)))
    (Class|StarChaserGameMode|SetBrightStarTrue _asstar_chaser_game_mode 1)
    (bind _returnvalue_2 (Class|StarChaserGameMode|GetTotalStars _asstar_chaser_game_mode))
    (Class|StarChaserGameMode|SetTotalStars _asstar_chaser_game_mode (+ _returnvalue_2 100))
    (bind _returnvalue_3 (Class|StarChaserGameMode|GetCurrentStars _asstar_chaser_game_mode))
    (Class|StarChaserGameMode|SetCurrentStars _asstar_chaser_game_mode (+ _returnvalue_3 100))
    (Class|StarChaserGameMode|Save _asstar_chaser_game_mode)
    (Audio|SpawnSound2D "/Game/Audio/chime_tinkle_wood_bell_positive_05.chime_tinkle_wood_bell_positive_05" 1.0 1.0 0.0 0)
    (Actor|DestroyActor)))

(fn ConstructionScript)
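; BP_StarPickUp is a star collectible power-up for an endless runner that adds to the game mode's Stars and the saved TotalStars.
; With the character's magnet active, a timeline and VInterpTo pull the star toward the player while it counts, sets Used, and saves after a delay.
; A second pickup chain counts, saves and destroys immediately unless Used is set.
; Neither chain has a triggering event wired, so neither runs as shown.
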(fn ConstructionScript)
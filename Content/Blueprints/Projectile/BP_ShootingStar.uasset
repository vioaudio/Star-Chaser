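; BP_ShootingStar is a projectile actor with a collision component and projectile movement.
; It destroys itself when the projectile movement stops.
; An unconnected chain, which never runs, would check the collision for overlapping Destructible objects and, while Counter is below one, play a block explosion sound and spawn BP_Explosion.
; Tick and the construction script are empty.
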(event OnProjectileStop(ProjectileMovement)
  (params (ImpactResult :type Hit%20Result%20Structure%20%28by%20ref%29))
  (Actor|DestroyActor))

(event EventTick
  (params (DeltaSeconds :type Float%20%28single-precision%29)))

(fn ConstructionScript)
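; BP_CloudPlatformB is a cloud platform obstacle that spawns a flying box and a bright star.
; On BeginPlay it spawns BP_FlyingBox1 at the ObstacleSpawn component's transform.
; Each Tick it polls the Box component for overlapping Pawns, and a hit spawns BP_BrightStar5 at the Sphere's transform, with Counter limiting this to one spawn.
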(event EventBeginPlay
  (Game|SpawnActorfromClass "/Game/Blueprints/Obstacles/BP_FlyingBox1.BP_FlyingBox1_C" (Transformation|GetWorldTransform (Variables|Default|GetObstacleSpawn)) "Undefined" 0 0))

(event EventTick
  (params (DeltaSeconds :type Float%20%28single-precision%29))
  (bind _counter (Variables|Default|GetCounter))
  (bind _box (Variables|Default|GetBox))
  ;[1 1 1] BrightStar Spawn
  (bind _returnvalue (Collision|ComponentOverlapActors _box (Transformation|GetWorldTransform _box) (Utilities|Array|MakeArray "ObjectTypeQuery3") 0))
  (if _returnvalue
    (if (< _counter 1)
      (Game|SpawnActorfromClass "/Game/Blueprints/BrightStars/BP_BrightStar5.BP_BrightStar5_C" (Transformation|GetWorldTransform (Variables|Default|GetSphere)) "Undefined" 0 0)
      (Math|Integer|IncrementInt _counter))))

(fn ConstructionScript)
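; BP_CloudPlatformA is a cloud platform obstacle that spawns a star when a pawn enters its trigger area.
; Every Tick polls the Box component with a component overlap query for Pawn objects instead of using overlap events.
; On the first hit it spawns BP_BrightStar3 at the Sphere component's transform, and a Counter variable blocks any further spawns.
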(event EventBeginPlay)

(event Collision|EventActorBeginOverlap
  (params (OtherActor :type Actor%20Object%20Reference)))

(event EventTick
  (params (DeltaSeconds :type Float%20%28single-precision%29))
  (bind _counter (Variables|Default|GetCounter))
  (bind _box (Variables|Default|GetBox))
  (bind _returnvalue (Collision|ComponentOverlapActors _box (Transformation|GetWorldTransform _box) (Utilities|Array|MakeArray "ObjectTypeQuery3") 0))
  (if _returnvalue
    (if (< _counter 1)
      (Game|SpawnActorfromClass "/Game/Blueprints/BrightStars/BP_BrightStar3.BP_BrightStar3_C" (Transformation|GetWorldTransform (Variables|Default|GetSphere)) "Undefined" 0 0)
      (Math|Integer|IncrementInt _counter))))

(fn ConstructionScript)
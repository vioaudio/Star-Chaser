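; BP_FlyingBox2 is an obstacle actor that moves along the world Y axis while rolling its mesh.
; On BeginPlay, the MoveBackForth timeline plays and each update adds its scaled value to the actor's Y location and StaticMesh1's roll.
; Both changes accumulate per update, so motion depends on frame rate.
; The rotation is read in world space but written as relative.
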(event EventBeginPlay
  (bind _returnvalue (Transformation|GetActorLocation))
  (bind _staticmesh1 (Variables|Default|GetStaticMesh1))
  (bind _returnvalue_2 (Transformation|GetWorldRotation _staticmesh1))
  ;[1 1 1] Spawn Movement
  (bind _moveback_forth (Timeline|MoveBack&Forth Play)
    (:Update
      (Transformation|SetActorLocation (Math|Vector|MakeVector (.x _returnvalue) (+ (.y _returnvalue) (* _moveback_forth 5.0)) (.z _returnvalue)) false false)
      (Transformation|SetRelativeRotation _staticmesh1 (Math|Rotator|MakeRotator (+ (.roll _returnvalue_2) (* _moveback_forth 1.0)) (.pitch _returnvalue_2) (.yaw _returnvalue_2)) false false))))

(fn ConstructionScript)
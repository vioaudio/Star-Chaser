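; Endless-runner floor tile that fills three lanes with hurdles, boxes, pickups and occasional cloud platforms on BeginPlay.
; SpawnObstacles cascades independent random rolls lane by lane; fairy spawns are disconnected.
; A cloud platform temporarily raises GameMode counters that suppress obstacle spawning on new tiles and further platforms.
; When the player overlaps its box, the tile requests another tile, awards points, raises run speed within limits, then destroys itself after a delay.
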(event OnComponentBeginOverlap(Box)
  (params (OverlappedComponent :type Primitive%20Component%20Object%20Reference) (OtherActor :type Actor%20Object%20Reference) (OtherComp :type Primitive%20Component%20Object%20Reference) (OtherBodyIndex :type Integer) (bFromSweep :type Boolean) (SweepResult :type Hit%20Result%20Structure%20%28by%20ref%29))
  ;[1 1 1] Spawn Floor
  (Utilities|Casting|CastToThirdPersonCharacter OtherActor)
  (bind _asthird_person_game_mode (Utilities|Casting|CastToThirdPersonGameMode (Game|GetGameMode)))
  (Default|SpawnTile _asthird_person_game_mode)
  (bind _asthird_person_game_mode_2 (Utilities|Casting|CastToThirdPersonGameMode (Game|GetGameMode)))
  (Variables|/Game/Blueprints/OldBP/ThirdPersonGameMode.ThirdPersonGameMode_C|SetCurrentPoints _asthird_person_game_mode_2 (+ 15 (Variables|/Game/Blueprints/OldBP/ThirdPersonGameMode.ThirdPersonGameMode_C|GetCurrentPoints _asthird_person_game_mode_2)))
  (bind _asthird_person_character (Utilities|Casting|CastToThirdPersonCharacter (Game|GetPlayerCharacter 0)))
  (Variables|/Script/Engine.CharacterMovementComponent|SetMaxWalkSpeed (Variables|/Script/Engine.Character|GetCharacterMovement _asthird_person_character) (Math|Float|Clamp(Float) (* (Variables|/Script/Engine.CharacterMovementComponent|GetMaxWalkSpeed (Variables|/Script/Engine.Character|GetCharacterMovement _asthird_person_character)) 1.01) 6e+02 1.2e+03))
  (Utilities|FlowControl|Delay 2.0)
  (Actor|DestroyActor))

(event EventBeginPlay
  ;[1 1 1] Spawn Obstacles
  (bind _asthird_person_game_mode (Utilities|Casting|CastToThirdPersonGameMode (Game|GetGameMode)))
  (if (> (Variables|/Game/Blueprints/OldBP/ThirdPersonGameMode.ThirdPersonGameMode_C|GetObjectDelay _asthird_person_game_mode) 0)
    (Development|PrintString (Utilities|String|ToString(Integer) (Variables|/Game/Blueprints/OldBP/ThirdPersonGameMode.ThirdPersonGameMode_C|GetObjectDelay _asthird_person_game_mode)))
    (else
      (Development|PrintString (Utilities|String|ToString(Integer) (Variables|/Game/Blueprints/OldBP/ThirdPersonGameMode.ThirdPersonGameMode_C|GetObjectDelay _asthird_person_game_mode)))
      (bind _cloudplatform (CallFunction|SpawnObstacles))
      (if _cloudplatform
        (bind _asthird_person_game_mode_2 (Utilities|Casting|CastToThirdPersonGameMode (Game|GetGameMode)))
        (bind _result (Math|Integer|IncrementInt (Variables|/Game/Blueprints/OldBP/ThirdPersonGameMode.ThirdPersonGameMode_C|GetObjectDelay _asthird_person_game_mode_2))
          (:%20%20
            (bind _result_2 (Math|Integer|IncrementInt (Variables|/Game/Blueprints/OldBP/ThirdPersonGameMode.ThirdPersonGameMode_C|GetCloudPlatCounter _asthird_person_game_mode_2))
              (:%20%20
                (Variables|/Game/Blueprints/OldBP/ThirdPersonGameMode.ThirdPersonGameMode_C|SetCloudPlatCounter _asthird_person_game_mode_2 _result_2)
                (Variables|/Game/Blueprints/OldBP/ThirdPersonGameMode.ThirdPersonGameMode_C|SetObjectDelay _asthird_person_game_mode_2 _result)
                (Utilities|FlowControl|Delay 3.0)
                (bind _asthird_person_game_mode_3 (Utilities|Casting|CastToThirdPersonGameMode (Game|GetGameMode)))
                (bind _result_3 (Math|Integer|DecrementInt (Variables|/Game/Blueprints/OldBP/ThirdPersonGameMode.ThirdPersonGameMode_C|GetObjectDelay _asthird_person_game_mode_3))
                  (:%20%20
                    (Variables|/Game/Blueprints/OldBP/ThirdPersonGameMode.ThirdPersonGameMode_C|SetObjectDelay _asthird_person_game_mode_3 _result_3)
                    (Utilities|FlowControl|Delay 7.0)
                    (bind _asthird_person_game_mode_4 (Utilities|Casting|CastToThirdPersonGameMode (Game|GetGameMode)))
                    (bind _result_4 (Math|Integer|DecrementInt (Variables|/Game/Blueprints/OldBP/ThirdPersonGameMode.ThirdPersonGameMode_C|GetCloudPlatCounter _asthird_person_game_mode_4))
                      (:%20%20
                        (Variables|/Game/Blueprints/OldBP/ThirdPersonGameMode.ThirdPersonGameMode_C|SetCloudPlatCounter _asthird_person_game_mode_4 _result_4)))))))))))))

(fn ConstructionScript)

(fn SpawnObstacles
  (bind _returnvalue (Math|Random|RandomFloatinRange 0.0 1.0))
  (bind _returnvalue_2 (Math|Random|RandomFloatinRange 0.0 1.0))
  (bind _returnvalue_3 (Math|Random|RandomFloatinRange 0.0 1.0))
  (bind _lane0 (Variables|Default|GetLane0))
  (bind _lane1 (Variables|Default|GetLane1))
  (bind _lane2 (Variables|Default|GetLane2))
  (bind _returnvalue_4 (Transformation|GetWorldTransform _lane0))
  (bind _returnvalue_5 (Transformation|GetWorldTransform _lane2))
  (bind _returnvalue_6 (Transformation|GetWorldTransform _lane1))
  ;[1 1 1] LANE0
  (if (Math|Float|InRange(Float) _returnvalue_2 0.0 0.2)
    (Game|SpawnActorfromClass "/Game/Blueprints/Obstacles/BP_Obstacle_Hurdle.BP_Obstacle_Hurdle_C" _returnvalue_4 "Undefined" 0 0)
    ;[1 1 1] LANE1
    (if (Math|Float|InRange(Float) _returnvalue_3 0.0 0.2) :!label _label
      (Game|SpawnActorfromClass "/Game/Blueprints/Obstacles/BP_Obstacle_Hurdle.BP_Obstacle_Hurdle_C" _returnvalue_6 "Undefined" 0 0)
      ;[1 1 1] LANE2
      (if (Math|Float|InRange(Float) _returnvalue 0.0 0.2) :!label _label_2
        (Game|SpawnActorfromClass "/Game/Blueprints/Obstacles/BP_Obstacle_Hurdle.BP_Obstacle_Hurdle_C" _returnvalue_5 "Undefined" 0 0)
        (elif (Math|Float|InRange(Float) _returnvalue 0.2 0.4)
          (Game|SpawnActorfromClass "/Game/Blueprints/Obstacles/BP_FlyingBox2.BP_FlyingBox2_C" _returnvalue_5 "Undefined" 0 0)
          (elif (Math|Float|InRange(Float) _returnvalue 0.4 0.5)
            (Game|SpawnActorfromClass "/Game/Blueprints/Obstacles/BP_Obstacle_Box.BP_Obstacle_Box_C" _returnvalue_5 "Undefined" 0 0)
            (elif (Math|Float|InRange(Float) _returnvalue 0.5 0.95)
              (Game|SpawnActorfromClass "/Game/Blueprints/PowerUps/BP_StarPickUp.BP_StarPickUp_C" _returnvalue_5 "Undefined" 0 0)
              (elif (Math|Float|InRange(Float) _returnvalue 0.95 0.975)
                (Game|SpawnActorfromClass "/Game/Blueprints/PowerUps/BP_MagnetPickup.BP_MagnetPickup_C" _returnvalue_5 "Undefined" 0 0)
                (elif (Math|Float|InRange(Float) _returnvalue 0.975 1.0)
                  (Game|SpawnActorfromClass "/Game/Blueprints/PowerUps/BP_BootsPickUp.BP_BootsPickUp_C" _returnvalue_5 "Undefined" 0 0)
                  (elif (not (Math|Float|InRange(Float) _returnvalue 0.755 0.76))
                    (if (not (Math|Float|InRange(Float) _returnvalue 0.76 0.765))
                      (if (not (Math|Float|InRange(Float) _returnvalue 0.765 0.77))
                        (if (not (Math|Float|InRange(Float) _returnvalue 0.77 0.775))
                          (if (Math|Float|InRange(Float) _returnvalue 0.775 0.78)
                            _)))))))))))
      (elif (Math|Float|InRange(Float) _returnvalue_3 0.4 0.5)
        (Game|SpawnActorfromClass "/Game/Blueprints/Obstacles/BP_Obstacle_Box.BP_Obstacle_Box_C" _returnvalue_6 "Undefined" 0 0)
        (elif (Math|Float|InRange(Float) _returnvalue_3 0.5 0.95)
          (Game|SpawnActorfromClass "/Game/Blueprints/PowerUps/BP_StarPickUp.BP_StarPickUp_C" _returnvalue_6 "Undefined" 0 0)
          (goto _label_2)
          (elif (Math|Float|InRange(Float) _returnvalue_3 0.95 0.975)
            (Game|SpawnActorfromClass "/Game/Blueprints/PowerUps/BP_MagnetPickup.BP_MagnetPickup_C" _returnvalue_6 "Undefined" 0 0)
            (goto _label_2)
            (elif (Math|Float|InRange(Float) _returnvalue_3 0.975 1.0)
              (Game|SpawnActorfromClass "/Game/Blueprints/PowerUps/BP_BootsPickUp.BP_BootsPickUp_C" _returnvalue_6 "Undefined" 0 0)
              (goto _label_2)
              (elif (not (Math|Float|InRange(Float) _returnvalue_3 0.755 0.76))
                (if (not (Math|Float|InRange(Float) _returnvalue_3 0.76 0.765))
                  (if (not (Math|Float|InRange(Float) _returnvalue_3 0.765 0.77))
                    (if (not (Math|Float|InRange(Float) _returnvalue_3 0.77 0.775))
                      (if (not (Math|Float|InRange(Float) _returnvalue_3 0.775 0.78))
                        ;[1 1 1] Cloud Platforms
                        (if (Math|Float|InRange(Float) _returnvalue_3 0.2 0.3)
                          (bind _asthird_person_game_mode (Utilities|Casting|CastToThirdPersonGameMode (Game|GetGameMode)))
                          (if (> 1 (Variables|/Game/Blueprints/OldBP/ThirdPersonGameMode.ThirdPersonGameMode_C|GetCloudPlatCounter _asthird_person_game_mode))
                            (Game|SpawnActorfromClass "/Game/Blueprints/Obstacles/BP_CloudPlatformA.BP_CloudPlatformA_C" _returnvalue_6 "Undefined" 0 0)
                            (return true))
                          (elif (Math|Float|InRange(Float) _returnvalue_3 0.3 0.4)
                            (bind _asthird_person_game_mode_2 (Utilities|Casting|CastToThirdPersonGameMode (Game|GetGameMode)))
                            (if (> 1 (Variables|/Game/Blueprints/OldBP/ThirdPersonGameMode.ThirdPersonGameMode_C|GetCloudPlatCounter _asthird_person_game_mode_2))
                              (Game|SpawnActorfromClass "/Game/Blueprints/Obstacles/BP_CloudPlatformB.BP_CloudPlatformB_C" _returnvalue_6 "Undefined" 0 0)
                              (return true))))))))))))))
    (elif (Math|Float|InRange(Float) _returnvalue_2 0.4 0.5)
      (Game|SpawnActorfromClass "/Game/Blueprints/Obstacles/BP_Obstacle_Box.BP_Obstacle_Box_C" _returnvalue_4 "Undefined" 0 0)
      (goto _label)
      (elif (Math|Float|InRange(Float) _returnvalue_2 0.2 0.3)
        (Game|SpawnActorfromClass "/Game/Blueprints/Obstacles/BP_FlyingBox1.BP_FlyingBox1_C" _returnvalue_4 "Undefined" 0 0)
        (elif (Math|Float|InRange(Float) _returnvalue_2 0.5 0.75)
          (Game|SpawnActorfromClass "/Game/Blueprints/PowerUps/BP_StarPickUp.BP_StarPickUp_C" _returnvalue_4 "Undefined" 0 0)
          (goto _label)
          (elif (Math|Float|InRange(Float) _returnvalue_2 0.95 0.975)
            (Game|SpawnActorfromClass "/Game/Blueprints/PowerUps/BP_MagnetPickup.BP_MagnetPickup_C" _returnvalue_4 "Undefined" 0 0)
            (goto _label)
            (elif (Math|Float|InRange(Float) _returnvalue_2 0.975 1.0)
              (Game|SpawnActorfromClass "/Game/Blueprints/PowerUps/BP_BootsPickUp.BP_BootsPickUp_C" _returnvalue_4 "Undefined" 0 0)
              (goto _label)
              (elif (not (Math|Float|InRange(Float) _returnvalue_2 0.755 0.76))
                (if (not (Math|Float|InRange(Float) _returnvalue_2 0.76 0.765))
                  (if (not (Math|Float|InRange(Float) _returnvalue_2 0.765 0.77))
                    (if (not (Math|Float|InRange(Float) _returnvalue_2 0.77 0.775))
                      (if (Math|Float|InRange(Float) _returnvalue_2 0.775 0.78)
                        _))))))))))))